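; BP_Tower_Area is a clickable actor, apparently a tower placement spot, that opens a UI widget when clicked.
; Its static mesh swaps materials on cursor hover, hover exit, click and release.
; Each click creates a new DefaultWidget for player 0, adds it to the viewport and sets Clicked.
; Clicked is never read here, so hover events still replace the clicked material.
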(event `self.ReceiveBeginPlay`
  (set `self.bClicked` false))

(event `self.StaticMesh.OnBeginCursorOver`
  (params (TouchedComponent :type "PrimitiveComponent Object Reference"))
  (`PrimitiveComponent.SetMaterial` (`self.StaticMesh`) 0 "/Game/Geometry/Meshes/CubeMaterial.CubeMaterial"))

(event `self.StaticMesh.OnEndCursorOver`
  (params (TouchedComponent :type "PrimitiveComponent Object Reference"))
  (`PrimitiveComponent.SetMaterial` (`self.StaticMesh`) 0 "/Game/StarterContent/Blueprints/Assets/M_LightStage_Skybox_Black.M_LightStage_Skybox_Black"))

(event `self.StaticMesh.OnClicked`
  (params (TouchedComponent :type "PrimitiveComponent Object Reference") (ButtonPressed :type "Key Structure"))
  (`PrimitiveComponent.SetMaterial` (`self.StaticMesh`) 0 "/Game/StarterContent/Materials/M_CobbleStone_Rough.M_CobbleStone_Rough")
  (bind _returnvalue (`|CreateWidget` "/Game/DefaultTest/Widget/DefaultWidget.DefaultWidget_C" (`GameplayStatics.GetPlayerController` 0)))
  (`UserWidget.AddToViewport` _returnvalue 0)
  (set `self.bClicked` true))

(event `self.StaticMesh.OnReleased`
  (params (TouchedComponent :type "PrimitiveComponent Object Reference") (ButtonReleased :type "Key Structure"))
  (`PrimitiveComponent.SetMaterial` (`self.StaticMesh`) 0 "/Game/StarterContent/Materials/M_CobbleStone_Rough.M_CobbleStone_Rough"))

(fn `UserConstructionScript`)